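; Paper golf player controller that turns Enhanced Input into shot aiming, flicking, camera look and pause actions.
; Turn activation and spectating swap mapping contexts, while guard functions gate each action; shoot also skips the hole flyby, with a debounce.
; Aim changes refresh a visible ShotArcPreviewComponent arc, whose adjustable target power feeds the HUD.
; The arc auto-shows after a short delay when a turn's initial rotation is near zero; debug keys handle stats, debug draw and recording.
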(event Custom|Shoot%20Debounce%20Expired
  ;[1 1 1] Shoot Controls
  (Variables|Default|SetShoot%20Debounce false))

(event Input|EnhancedActionEvents|EnhancedInputActionIA_FlickLocZ
  (params (ActionValue :type Float%20%28double-precision%29) (ElapsedSeconds :type Float%20%28double-precision%29) (TriggeredSeconds :type Float%20%28double-precision%29) (InputAction :type Input%20Action%20Object%20Reference :default "/Game/Blueprints/Player/Input/IA_FlickLocZ.IA_FlickLocZ"))
  ;[1 1 1] Shoot Controls
  (if (and (CallFunction|ShouldProcessInput) (not (CallFunction|IsinLookMode)))
    (Class|GolfPlayerController|ProcessFlickZInput ActionValue)
    (CallFunction|UpdateShotPreview)))

(event Input|EnhancedActionEvents|EnhancedInputActionIA_Shoot
  (params (ActionValue :type Boolean) (ElapsedSeconds :type Float%20%28double-precision%29) (TriggeredSeconds :type Float%20%28double-precision%29) (InputAction :type Input%20Action%20Object%20Reference :default "/Game/Blueprints/Player/Input/IA_Shoot.IA_Shoot"))
  ;[1 1 1] Shoot Controls
  (:Started
    (if (not (Variables|Default|GetShoot%20Debounce))
      (if (CallFunction|ShouldProcessInput)
        (Class|ShotArcPreviewComponent|HideShotArc (Variables|Default|GetShotArcPreviewComponent))
        (Class|GolfPlayerController|ProcessShootInput)
        (elif (Class|GolfPlayerController|IsinCinematicSequence)
          (Class|GolfPlayerController|SkipHoleFlybyandCameraIntroduction)
          (Variables|Default|SetShoot%20Debounce true)
          (Utilities|Time|SetTimerbyEvent (delegate Custom|Shoot%20Debounce%20Expired) (Variables|Default|GetShoot%20Debounce%20Time)))))))

(event Input|EnhancedActionEvents|EnhancedInputActionIA_TargetShotPower_Decrease
  (params (ActionValue :type Boolean) (ElapsedSeconds :type Float%20%28double-precision%29) (TriggeredSeconds :type Float%20%28double-precision%29) (InputAction :type Input%20Action%20Object%20Reference :default "/Game/Blueprints/Player/Input/IA_TargetShotPower_Decrease.IA_TargetShotPower_Decrease"))
  ;[1 1 1] Shot Preview
  (if (CallFunction|ShouldProcessTargetShotPowerChange)
    (CallFunction|UpdateTargetPower (* (Variables|Default|GetTarget%20Shot%20Power%20Scroll%20Delta) -1.0))
    (CallFunction|UpdateShotPreview)))

(event Input|EnhancedActionEvents|EnhancedInputActionIA_Look
  (params (ActionValue :type Vector%202D%20Structure) (ElapsedSeconds :type Float%20%28double-precision%29) (TriggeredSeconds :type Float%20%28double-precision%29) (InputAction :type Input%20Action%20Object%20Reference :default "/Game/Blueprints/Player/Input/IA_Look.IA_Look"))
  ;[1 1 1] Look Controls
  (if (CallFunction|ShouldProcessLookInput)
    (Class|PlayerController|AddYawInput (.x ActionValue))
    (Class|PlayerController|AddPitchInput (.y ActionValue))))

(event Input|EnhancedActionEvents|EnhancedInputActionIA_Look_Reset
  (params (ActionValue :type Boolean) (ElapsedSeconds :type Float%20%28double-precision%29) (TriggeredSeconds :type Float%20%28double-precision%29) (InputAction :type Input%20Action%20Object%20Reference :default "/Game/Blueprints/Player/Input/IA_Look_Reset.IA_Look_Reset"))
  ;[1 1 1] Look Controls
  (if (CallFunction|ShouldProcessLookInput)
    (Class|GolfPlayerController|ResetCameraRotation)))

(event Input|EnhancedActionEvents|EnhancedInputActionIA_Look_Zoom
  (params (ActionValue :type Float%20%28double-precision%29) (ElapsedSeconds :type Float%20%28double-precision%29) (TriggeredSeconds :type Float%20%28double-precision%29) (InputAction :type Input%20Action%20Object%20Reference :default "/Game/Blueprints/Player/Input/IA_Look_Zoom.IA_Look_Zoom"))
  ;[1 1 1] Look Controls
  (if (CallFunction|ShouldProcessZoom)
    (Class|GolfPlayerController|AddCameraZoomDelta ActionValue)))

(event Input|EnhancedActionEvents|EnhancedInputActionIA_RotateZ
  (params (ActionValue :type Float%20%28double-precision%29) (ElapsedSeconds :type Float%20%28double-precision%29) (TriggeredSeconds :type Float%20%28double-precision%29) (InputAction :type Input%20Action%20Object%20Reference :default "/Game/Blueprints/Player/Input/IA_RotateZ.IA_RotateZ"))
  ;[1 1 1] Rotation Controls
  (if (CallFunction|ShouldProcessInput)
    (Class|GolfPlayerController|AddPaperGolfPawnRelativeRotation (Math|Rotator|MakeRotator 0.0 0.0 ActionValue))
    (CallFunction|UpdateShotPreview)))

(event Input|EnhancedActionEvents|EnhancedInputActionIA_TiltX
  (params (ActionValue :type Float%20%28double-precision%29) (ElapsedSeconds :type Float%20%28double-precision%29) (TriggeredSeconds :type Float%20%28double-precision%29) (InputAction :type Input%20Action%20Object%20Reference :default "/Game/Blueprints/Player/Input/IA_TiltX.IA_TiltX"))
  ;[1 1 1] Rotation Controls
)

(event Input|EnhancedActionEvents|EnhancedInputActionIA_Tilty
  (params (ActionValue :type Float%20%28double-precision%29) (ElapsedSeconds :type Float%20%28double-precision%29) (TriggeredSeconds :type Float%20%28double-precision%29) (InputAction :type Input%20Action%20Object%20Reference :default "/Game/Blueprints/Player/Input/IA_Tilty.IA_Tilty"))
  ;[1 1 1] Rotation Controls
  (if (CallFunction|ShouldProcessInput)
    (Class|GolfPlayerController|AddPaperGolfPawnRelativeRotation (Math|Rotator|MakeRotator 0.0 ActionValue 0.0))
    (CallFunction|UpdateShotPreview)))

(event Input|EnhancedActionEvents|EnhancedInputActionIA_ResetShot
  (params (ActionValue :type Boolean) (ElapsedSeconds :type Float%20%28double-precision%29) (TriggeredSeconds :type Float%20%28double-precision%29) (InputAction :type Input%20Action%20Object%20Reference :default "/Game/Blueprints/Player/Input/IA_ResetShot.IA_ResetShot"))
  ;[1 1 1] Shoot Controls
  (:Started
    (if (CallFunction|ShouldProcessInput)
      (Class|ShotArcPreviewComponent|HideShotArc (Variables|Default|GetShotArcPreviewComponent))
      (Class|GolfPlayerController|ResetShotwithServerInvocation))))

(event Input|EnhancedActionEvents|EnhancedInputActionIA_Pause
  (params (ActionValue :type Boolean) (ElapsedSeconds :type Float%20%28double-precision%29) (TriggeredSeconds :type Float%20%28double-precision%29) (InputAction :type Input%20Action%20Object%20Reference :default "/Game/Blueprints/Player/Input/IA_Pause.IA_Pause"))
  (:Completed
    (CallFunction|OnPausePressed)))

(event Input|EnhancedActionEvents|EnhancedInputActionIA_ToggleShot
  (params (ActionValue :type Boolean) (ElapsedSeconds :type Float%20%28double-precision%29) (TriggeredSeconds :type Float%20%28double-precision%29) (InputAction :type Input%20Action%20Object%20Reference :default "/Game/Blueprints/Player/Input/IA_ToggleShot.IA_ToggleShot"))
  ;[1 1 1] Shoot Controls
  (:Started
    (if (CallFunction|ShouldProcessInput)
      (Class|GolfPlayerController|ToggleShotType)
      (CallFunction|UpdateShotPreview))))

(event Input|EnhancedActionEvents|EnhancedInputActionIA_ShotPreview
  (params (ActionValue :type Boolean) (ElapsedSeconds :type Float%20%28double-precision%29) (TriggeredSeconds :type Float%20%28double-precision%29) (InputAction :type Input%20Action%20Object%20Reference :default "/Game/Blueprints/Player/Input/IA_ShotPreview.IA_ShotPreview"))
  ;[1 1 1] Shot Preview
  (:Started
    (if (CallFunction|ShouldProcessInput)
      (if (CallFunction|IsinShotPreview)
        (Class|ShotArcPreviewComponent|HideShotArc (Variables|Default|GetShotArcPreviewComponent))
        (else
          (CallFunction|ShowShotPreview))))))

(event Input|EnhancedActionEvents|EnhancedInputActionIA_TargetShotPower_Increase
  (params (ActionValue :type Boolean) (ElapsedSeconds :type Float%20%28double-precision%29) (TriggeredSeconds :type Float%20%28double-precision%29) (InputAction :type Input%20Action%20Object%20Reference :default "/Game/Blueprints/Player/Input/IA_TargetShotPower_Increase.IA_TargetShotPower_Increase"))
  ;[1 1 1] Shot Preview
  (if (CallFunction|ShouldProcessTargetShotPowerChange)
    (CallFunction|UpdateTargetPower (Variables|Default|GetTarget%20Shot%20Power%20Scroll%20Delta))
    (CallFunction|UpdateShotPreview)))

(event EventBeginPlay
  (CallFunction|InitializeInput))

(event EventBlueprintResetShot
  ;[1 1 1] Shoot Controls
  (CallFunction|ResetTargetShotPower))

(event EventBlueprintSpectate
  (params (InPawn :type Paper%20Golf%20Pawn%20Object%20Reference) (InPlayerState :type Golf%20Player%20State%20Object%20Reference))
  (CallFunction|DisableInput))

(event EventBlueprintActivateTurn
  (CallFunction|InitializeInput))

(event EventBlueprintPlayerReadyforShot
  (params (InitialRelativeRotation :type Rotator%20%28by%20ref%29 :default "0, 0, 0"))
  ;[1 1 1] Shot Preview
  (if (CallFunction|ShouldShowShotPreviewonTurnActivation InitialRelativeRotation)
    (Utilities|FlowControl|Delay 0.1) ; Avoid drawing artifacts with camera not quite set yet
    (CallFunction|ShowShotPreview)))

(event Input|KeyboardEvents|DebugKeyF12
  (params (Key :type Key%20Structure) (ActionValue :type Input%20Action%20Value%20Structure))
  ;[1 1 1] Debug
  (:Pressed
    (CallFunction|ToggleDebugDisplay)))

(event Input|KeyboardEvents|DebugKeyF7
  (params (Key :type Key%20Structure) (ActionValue :type Input%20Action%20Value%20Structure))
  ;[1 1 1] Debug
  (:Pressed
    (if (Class|VisualLoggerUtils|IsRecording)
      (Class|VisualLoggerUtils|StopRecording)
      (else
        (Class|VisualLoggerUtils|StartRecording)))))

(event Input|KeyboardEvents|DebugKeyF6
  (params (Key :type Key%20Structure) (ActionValue :type Input%20Action%20Value%20Structure))
  ;[1 1 1] Debug
  (:Pressed
    (CallFunction|ShowStats)))

(fn ConstructionScript)

(fn InitializeInput
  (bind _self self)
  (bind _returnvalue (PlayerController|LocalPlayerSubsystems|GetEnhancedInputLocalPlayerSubsystem _self))
  (Utilities|IsValid _returnvalue
    (:Is%20Valid
      (Input|RemoveMappingContext _returnvalue "/Game/Blueprints/Player/Input/IMC_ShotSpectator.IMC_ShotSpectator" "(bIgnoreAllPressedKeysUntilRelease=True,bForceImmediately=False,bNotifyUserSettings=False)")
      (Input|AddMappingContext _returnvalue "/Game/Blueprints/Player/Input/IMC_Default.IMC_Default" 0 "(bIgnoreAllPressedKeysUntilRelease=True,bForceImmediately=False,bNotifyUserSettings=False)"))))

(fn ShowTutorial
  (if (not (Class|TutorialTrackingSubsystem|IsTutorialSeen (Subsystems|GetTutorialTrackingSubsystem)))
    (bind _golf_hud (Utilities|GetPaperGolfHUDChecked self)
      (:Valid
        (Class|PGHUD|DisplayMessageWidget _golf_hud "Tutorial")))))

(fn ShowStats
  (if (Class|BuildUtilities|IsNotShipping)
    (Development|ExecuteConsoleCommand "stat fps" 0)
    (Development|ExecuteConsoleCommand "stat unit" 0)))

(fn ToggleDebugDisplay
  (if (Class|BuildUtilities|IsNotShipping)
    (Variables|Default|SetDebug%20Draw (not (Variables|Default|GetDebug%20Draw)))))

(fn IsDebugDrawEnabled
  (return (Variables|Default|GetDebug%20Draw)))

(fn ShouldProcessInput
  (return (and (Class|GolfPlayerController|CanFlick) (Class|GolfPlayerController|IsInputEnabled))))

(fn ShowShotPreview
  (Class|ShotArcPreviewComponent|ShowShotArc (Variables|Default|GetShotArcPreviewComponent) (Utilities|Struct|MakeFlickParams (Class|GolfPlayerController|GetShotType) (Class|GolfPlayerController|GetFlickZ) (Variables|Default|GetTarget%20Shot%20Power%20Fraction) 0.0))
  (CallFunction|UpdateTargetPower 0.0))

(fn UpdateShotPreview
  (if (CallFunction|IsinShotPreview)
    (CallFunction|ShowShotPreview)))

(fn ResetTargetShotPower
  (Variables|Default|SetTarget%20Shot%20Power%20Fraction 1.0))

(fn ShouldProcessTargetShotPowerChange
  (return (and (CallFunction|ShouldProcessInput) (CallFunction|IsinShotPreview))))

(fn UpdateTargetPower
  (params (Delta%20Amount :type Float%20%28double-precision%29))
  (Variables|Default|SetTarget%20Shot%20Power%20Fraction (Math|Float|Clamp(Float) (+ (Variables|Default|GetTarget%20Shot%20Power%20Fraction) Delta%20Amount)))
  (bind _asbp_golf_hud (Utilities|Casting|CastToBP_Golf_HUD (HUD|GetHUD)))
  (Utilities|IsValid (Class|PGHUD|GetGolfWidget _asbp_golf_hud)
    (:Is%20Valid
      (Class|GolfUserWidget|SetTargetPower (Class|PGHUD|GetGolfWidget _asbp_golf_hud) (Variables|Default|GetTarget%20Shot%20Power%20Fraction)))))

(fn ShouldProcessZoom
  (return (and (CallFunction|ShouldProcessLookInput) (not (CallFunction|IsinShotPreview)))))

(fn IsinShotPreview
  (return (Class|ShotArcPreviewComponent|IsVisible (Variables|Default|GetShotArcPreviewComponent))))

(fn IsinLookMode
  (return (or (Input|EnhancedActionValues|GetIA_Look_Activation) (not (Math|Float|NearlyEqual(Float) (Input|EnhancedActionValues|GetIA_Look_Zoom) 0.0 1e-06)))))

(fn OnPausePressed
  (if (not (Class|BasePlayerController|IsPauseActionActive))
    (bind _returnvalue (UserInterface|CreateWidget "/Game/Blueprints/UI/Menus/PauseMenu.PauseMenu_C" 0 (select (Class|BasePlayerController|CanPauseGame) "Resume" "Close")))
    (Utilities|IsValid _returnvalue
      (:Is%20Valid
        (UserInterface|Viewport|AddtoViewport _returnvalue 0)
        (Class|BasePlayerController|PauseGame 0)))))

(fn DisableInput
  (bind _self self)
  (bind _returnvalue (PlayerController|LocalPlayerSubsystems|GetEnhancedInputLocalPlayerSubsystem _self))
  (Utilities|IsValid _returnvalue
    (:Is%20Valid
      (Input|RemoveMappingContext _returnvalue "/Game/Blueprints/Player/Input/IMC_Default.IMC_Default" "(bIgnoreAllPressedKeysUntilRelease=True,bForceImmediately=False,bNotifyUserSettings=False)")
      (Input|AddMappingContext _returnvalue "/Game/Blueprints/Player/Input/IMC_ShotSpectator.IMC_ShotSpectator" 0 "(bIgnoreAllPressedKeysUntilRelease=True,bForceImmediately=False,bNotifyUserSettings=False)"))))

(fn ShouldProcessLookInput
  (return (or (CallFunction|ShouldProcessInput) (Class|GolfPlayerController|IsSpectatingShotSetup))))

(fn ShouldShowShotPreviewonTurnActivation
  (params (Initial%20Shot%20Rotation :type Rotator))
  (if (Utilities|Operators|EqualEqual :A Initial%20Shot%20Rotation :ErrorTolerance 1.0)
    (return true) ; Show if initial pitch angle not set as then there is probably\nan obstacle that requires finesse
  ))
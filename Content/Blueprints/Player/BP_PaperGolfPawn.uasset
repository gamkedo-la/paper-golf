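; Paper golf player pawn Blueprint that handles player color tinting and an overhead-style player indicator in multiplayer.
; Replicated PlayerColor drives a lazily created dynamic material on the golf mesh through its RepNotify.
; TurnStarted, set by turn and shot events, triggers a RepNotify that hides the indicator during the turn and otherwise shows it for the possessing player state.
; The indicator component is async-loaded on first use, skipping dedicated servers and single-player games.
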(event `self.OnTurnStarted`
  (set `self.Turn Started` true))

(event `self.OnShotFinished`
  (set `self.Turn Started` false))

(event `self.SetPawnColor`
  (params (Color :type "LinearColor Structure (by ref)"))
  ;[1 1 1] Set Pawn Color
  (set `self.Player Color` Color))

(event `Toggle Player Indicator Async`
  (`self.Toggle Player Indicator`))

(event `self.ReceivePossessed`
  (params (NewController :type "Controller Object Reference"))
  (bind _asgolf_player_state (cast `GolfPlayerState` (`self.PlayerState`)))
  (set `self.PlayerIndicatorState` _asgolf_player_state))

(fn `OnRep_Player Color`
  (`self.Set Player Color` (`self.Player Color`)))

(fn `OnRep_Turn Started`
  (`self.Toggle Player Indicator Async`))

(fn `Set Player Color`
  (params (Color :type "LinearColor Structure"))
  (bind _papergolfmesh (`self.PaperGolfMesh`))
  (`/Engine/EditorBlueprintResources/StandardMacros.IsValid` (`self.Player Color MID`)
    (:`Is Valid`
      _)
    (:`Is Not Valid`
      (bind _returnvalue (`PrimitiveComponent.CreateDynamicMaterialInstance` _papergolfmesh 0 (`PrimitiveComponent.GetMaterial` _papergolfmesh 0) "None"))
      (bind _output_get (set `self.Player Color MID` _returnvalue))))
  (`MaterialInstanceDynamic.SetVectorParameterValue` _output_get "Tint" Color))

(fn `UserConstructionScript`)
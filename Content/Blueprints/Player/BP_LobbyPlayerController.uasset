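; BP_LobbyPlayerController is the lobby player controller, handling input setup and the pause menu.
; On BeginPlay it adds IMC_Default to the local player's Enhanced Input subsystem.
; Completing IA_Pause creates a pause menu widget with a "Close" resume option and switches to UI input mode, unless a menu is already active.
; BlueprintResumeGame clears the stored menu reference so the menu can open again.
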(event `self.ReceiveBeginPlay`
  (`self.Initialize Input`))

(event `EnhancedInput|/Game/Blueprints/Player/Input/IA_Pause`
  (params (ActionValue :type Boolean) (ElapsedSeconds :type "Float (double-precision)") (TriggeredSeconds :type "Float (double-precision)") (InputAction :type "InputAction Object Reference" :default "/Game/Blueprints/Player/Input/IA_Pause.IA_Pause"))
  (:`Completed`
    (`self.On Pause Pressed`)))

(event `self.BlueprintResumeGame`
  (set `self.Active Pause Menu` null))

(fn `Initialize Input`
  (bind _returnvalue (pcsubsystem `EnhancedInputLocalPlayerSubsystem` self))
  (`/Engine/EditorBlueprintResources/StandardMacros.IsValid` _returnvalue
    (:`Is Valid`
      (`EnhancedInputSubsystemInterface.AddMappingContext` _returnvalue "/Game/Blueprints/Player/Input/IMC_Default.IMC_Default" 0 (struct)))))

(fn `On Pause Pressed`
  (`/Engine/EditorBlueprintResources/StandardMacros.IsValid` (`self.Active Pause Menu`)
    (:`Is Not Valid`
      (bind _returnvalue (`|CreateWidget` "/Game/Blueprints/UI/Menus/PauseMenu.PauseMenu_C" null "Close"))
      (`/Engine/EditorBlueprintResources/StandardMacros.IsValid` _returnvalue
        (:`Is Valid`
          (set `self.Active Pause Menu` _returnvalue)
          (`UserWidget.AddToViewport` _returnvalue 0)
          (`self.SetInputModeUI` null))))))

(fn `UserConstructionScript`)
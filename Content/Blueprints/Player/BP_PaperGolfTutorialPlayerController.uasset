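; Player controller Blueprint for the paper golf tutorial, extending the base paper golf player controller.
; It overrides the check for showing the shot preview when a turn activates, hiding it while the player state reports zero shots taken.
; After the first shot it defers to the parent's decision.
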(fn `Should Show Shot Preview On Turn Activation`
  (params (`Initial Shot Rotation` :type "Rotator Structure"))
  (returns (Result :type Boolean))
  (if (== (`GolfPlayerState.GetShots` (`/Game/Blueprints/Library/BP_Utilities.Get Paper Golf Player State`)) 0)
    (return false) ; Don't show the shot preview on the first shot in the tutorial
    (else
      (return (`parent.Should Show Shot Preview On Turn Activation` `Initial Shot Rotation`)))))

(fn `UserConstructionScript`
  (`parent.UserConstructionScript`))
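; BP_GolfHole is the golf hole actor that detects when a paper golf pawn comes to rest inside it.
; Overlapping the hole collider stores the pawn and starts a looping timer that polls whether it is at rest; leaving clears the pawn.
; A resting pawn triggers OnScored on its player controller and stops the timer.
; BeginPlay creates a dynamic hole material and caches its color, which is not changed here.
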(event `self.ReceiveBeginPlay`
  (`self.InitMaterialInstance`))

(event `self.HoleCollider.OnComponentBeginOverlap`
  (params (OverlappedComponent :type "PrimitiveComponent Object Reference") (OtherActor :type "Actor Object Reference") (OtherComp :type "PrimitiveComponent Object Reference") (OtherBodyIndex :type Integer) (bFromSweep :type Boolean) (SweepResult :type "HitResult Structure (by ref)"))
  (bind _asbp_flicker_pawn (cast `/Game/Blueprints/Player/BP_PaperGolfPawn` OtherActor))
  (set `self.Flicker` _asbp_flicker_pawn)
  (bind _returnvalue (`KismetSystemLibrary.K2_SetTimerDelegate` (delegate `Check Scored Event`) 0.1 true))
  (set `self.Score Timer Handle` _returnvalue))

(event `self.HoleCollider.OnComponentEndOverlap`
  (params (OverlappedComponent :type "PrimitiveComponent Object Reference") (OtherActor :type "Actor Object Reference") (OtherComp :type "PrimitiveComponent Object Reference") (OtherBodyIndex :type Integer))
  (if (== OtherActor (`self.Flicker`))
    (set `self.Flicker` null)))

(event `Check Scored Event`
  (bind _scored (`self.On Score Timer Check`))
  (if _scored
    (`KismetSystemLibrary.K2_ClearAndInvalidateTimerHandle` (`self.Score Timer Handle`))))

(fn `Check Scored`
  (returns (Scored :type Boolean))
  (return (`PaperGolfPawn.IsAtRest` (`self.Flicker`))))

(fn `InitMaterialInstance`
  (bind _returnvalue (`PrimitiveComponent.CreateDynamicMaterialInstance` (`self.Mesh`) 0 "/Game/Materials/MI_Golf_Hole.MI_Golf_Hole" (`self.ColorParameterName`)))
  (bind _output_get (set `self.Hole MID` _returnvalue))
  (bind _returnvalue_2 (`MaterialInstanceDynamic.K2_GetVectorParameterValue` _output_get (`self.ColorParameterName`)))
  (bind _output_get_2 (set `self.CurrentMaterialColor` _returnvalue_2))
  (set `self.OriginalMaterialColor` _output_get_2))

(fn `On Score Timer Check`
  (returns (Scored :type Boolean))
  (bind _scored (`self.Check Scored`))
  (`/Engine/EditorBlueprintResources/StandardMacros.IsValid` (`self.Flicker`)
    (:`Is Valid`
      (if _scored
        (if _scored
          (bind _asbp_flicker_player_controller (cast `/Game/Blueprints/Player/BP_PaperGolfPlayerController` (`Pawn.GetController` (`self.Flicker`))))
          (`/Engine/EditorBlueprintResources/StandardMacros.IsValid` _asbp_flicker_player_controller
            (:`Is Valid`
              (`GolfPlayerController.OnScored` _asbp_flicker_player_controller)
              (return true))))))))

(fn `UserConstructionScript`)
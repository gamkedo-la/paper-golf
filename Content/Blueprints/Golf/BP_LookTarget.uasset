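; BP_LookTarget is a golf look target that exposes a hole number, a minimum 2D distance and a view-angle limit.
; BeginPlay converts MaxAngle in degrees to a cached cosine, returned as the minimum cosine angle, which suits dot-product angle checks.
; Simple getters expose these values, and IsHole always returns false, marking this target as something other than a hole.
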(event `self.ReceiveBeginPlay`
  (set `self.Cos Angle` (`KismetMathLibrary.DegCos` (`self.Max Angle`))))

(fn `GetHoleNumber`
  (returns (ReturnValue :type Integer))
  (return (`self.Hole Number`)))

(fn `GetMinCosAngle`
  (returns (ReturnValue :type "Float (single-precision)"))
  (return (`self.Cos Angle`)))

(fn `GetMinDistance2D`
  (returns (ReturnValue :type "Float (single-precision)"))
  (return (`self.Min Distance`)))

(fn `IsHole`
  (returns (ReturnValue :type Boolean))
  (return false))

(fn `UserConstructionScript`)
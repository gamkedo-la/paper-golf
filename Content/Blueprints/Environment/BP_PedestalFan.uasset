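; Pedestal fan environment actor with oscillation, spinning blades and an influence collider.
; On authority, BeginPlay registers the Influence collider and plays the FanOscillation.
; Blade spin is cosmetic and runs on clients too, via a looping timer applying a local rotation precomputed from axis, revolutions per second and timer interval.
; GetAirflowOriginAndDirection returns zero vectors, and the rotation calculation is flagged as not working.
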(event `self.ReceiveBeginPlay`
  (`|ExecutionSequence`
    (:`then_0`
      (`/Engine/EditorBlueprintResources/ActorMacros.Switch Has Authority`
        (:`Authority`
          (`self.SetInfluenceCollider` (`self.Influence`))
          (`Timeline|Fan Oscillation`))))
    (:`then_1`
      (set `self.Rotation Per Update` (`self.Calculate Rotation Per Update`))
      (`KismetSystemLibrary.K2_SetTimerDelegate` (delegate `Blade Rotation`) (`self.Blade Rotation Frequency`) true true))))

(event `Blade Rotation`
  (`SceneComponent.K2_AddLocalRotation` (`self.Fan Blades`) (`self.Rotation Per Update`) false false))

(fn `Calculate Rotation Per Update`
  (returns (`Rotation per update` :type "Rotator Structure"))
  (bind (_returnvalue_x _returnvalue_y _returnvalue_z) (`KismetMathLibrary.BreakVector` (* (`self.Blade Axis of Rotation`) (* (* (`self.Blade Revolutions Per Second`) 360.0) (`self.Blade Rotation Frequency`)))))
  (return (`KismetMathLibrary.MakeRotator` _returnvalue_x _returnvalue_y _returnvalue_z)))

(fn `GetAirflowOriginAndDirection`
  (returns (OutOrigin :type "Vector Structure") (OutDirection :type "Vector Structure"))
  (return (0.0 0.0 0.0) (0.0 0.0 0.0)))

(fn `UserConstructionScript`)
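; BP_OutOfBounds is an environment hazard Blueprint whose graphs keep its out-of-bounds text turned toward the local player's camera.
; On BeginPlay, unless on a dedicated server, it starts a looping timer at TextUpdateInterval when that value is non-negative.
; Each tick of the timer applies a look-at rotation toward the camera, following yaw, clamping pitch between MinPitch and MaxPitch, and preserving roll.
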(event `self.ReceiveBeginPlay`
  (if (>= (`self.Text Update Interval`) 0.0)
    (if (not (`KismetSystemLibrary.IsDedicatedServer`))
      (`KismetSystemLibrary.K2_SetTimer` null "Rotate Text Toward Camera" (`self.Text Update Interval`) true))))

(fn `Rotate Text Toward Camera`
  (locals (`Text Update Rate` :type "Float (double-precision)" :default 0.1) (`Camera Manager` :type "PlayerCameraManager Object Reference"))
  (bind _returnvalue (`PaperGolfGameUtilities.GetLocalPlayerCameraManager` null))
  (bind _text (`self.Text`))
  (bind _returnvalue_roll (`KismetMathLibrary.BreakRotator` (`SceneComponent.K2_GetComponentRotation` _text)))
  (bind (_returnvalue_roll_2 _returnvalue_pitch _returnvalue_yaw) (`KismetMathLibrary.BreakRotator` (`KismetMathLibrary.FindLookAtRotation` (`SceneComponent.K2_GetComponentLocation` _text) (`PlayerCameraManager.GetCameraLocation` _returnvalue))))
  (bind _output_get (set `local.Camera Manager` _returnvalue))
  (`/Engine/EditorBlueprintResources/StandardMacros.IsValid` _output_get
    (:`Is Valid`
      (`SceneComponent.K2_SetWorldRotation` _text (`KismetMathLibrary.MakeRotator` _returnvalue_roll (`KismetMathLibrary.FClamp` _returnvalue_pitch (`self.Min Pitch`) (`self.Max Pitch`)) _returnvalue_yaw) false false))))

(fn `UserConstructionScript`)
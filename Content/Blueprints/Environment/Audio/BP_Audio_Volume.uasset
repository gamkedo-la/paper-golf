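; BP_Audio_Volume is a trigger volume that plays its sound on actor overlap and fades it out when overlap ends.
; At BeginPlay it disables itself if no sound is set, or starts audio if the player pawn is already inside.
; Playback supports optional fade-in, random start time and restarting during a fade-out.
; Audio state changes set an Active flag, which lets Tick mirror the game's pause state onto the sound.
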(event `self.ReceiveBeginPlay`
  (bind _success (`self.Init`))
  (if _success
    (add `AudioComponent.OnAudioPlayStateChanged` (`self.Sound`) (delegate `On Audio State Changed`))
    (`self.Check Overlap At Start`)))

(event `On Audio State Changed`
  (params (PlayState :type "EAudioComponentPlayState Enum" :default "Playing"))
  (switch `EAudioComponentPlayState` PlayState
    (:`Playing`
      (set `self.Active` true :!label _label))
    (:`Stopped`
      (set `self.Active` false))
    (:`FadingIn`
      (goto _label))))

(event `self.ReceiveActorBeginOverlap`
  (params (OtherActor :type "Actor Object Reference"))
  (`self.Start Audio`))

(event `self.ReceiveActorEndOverlap`
  (params (OtherActor :type "Actor Object Reference"))
  (`self.Fade Out Audio`))

(event `self.ReceiveTick`
  (params (DeltaSeconds :type "Float (single-precision)"))
  (`self.Check For Pause`))

(fn `Check For Pause`
  (if (`self.Active`)
    (if (`GameplayStatics.IsGamePaused`)
      (`self.Pause Audio`)
      (else
        (`self.Resume Audio`)))))

(fn `Check Overlap At Start`
  (if (`self.IsOverlappingActor` (`GameplayStatics.GetPlayerPawn` 0))
    (`self.Start Audio`)))

(fn `Fade Out Audio`
  (if (`self.Enabled`)
    (`AudioComponent.FadeOut` (`self.Sound`) (`self.Fade Out Time`) 0.0 "Linear")
    (set `self.Is Fading Out` true)))

(fn `Get Audio Start Time`
  (returns (`Start Time` :type "Float (double-precision)"))
  (bind _end_duration_override (`self.End Duration Override`))
  (bind _sound (`AudioComponent.Sound` (`self.Sound`)))
  (if (`self.Random Start Time`)
    (`/Engine/EditorBlueprintResources/StandardMacros.IsValid` _sound
      (:`Is Valid`
        (return (`KismetMathLibrary.RandomFloatInRange` 0.0 (select `bool` (> _end_duration_override 0.0) :`false` (`SoundBase.Duration` _sound) :`true` _end_duration_override :!type "Float (double-precision)")))))))

(fn `Init`
  (returns (Success :type Boolean))
  (if (and (`KismetSystemLibrary.IsValid` (`AudioComponent.Sound` (`self.Sound`))) (`self.Enabled`))
    (return true)
    (else
      (`self.SetActorTickEnabled` false)
      (set `self.Enabled` false)
      (return false))))

(fn `Pause Audio`
  (if (`self.Enabled`)
    (`AudioComponent.SetPaused` (`self.Sound`) true)))

(fn `Resume Audio`
  (if (`self.Enabled`)
    (`AudioComponent.SetPaused` (`self.Sound`) false)))

(fn `Start Audio`
  (bind _start_time (`self.Get Audio Start Time`))
  (bind _sound (`self.Sound`))
  (bind _fade_in_time (`self.Fade In Time`))
  (if (`self.Enabled`)
    (if (`AudioComponent.IsPlaying` (`self.Sound`))
      (if (`self.Is Fading Out`)
        (if (> _fade_in_time 0.0) :!label _label
          (`AudioComponent.FadeIn` _sound _fade_in_time 1.0 _start_time "Linear")
          (else
            (`AudioComponent.Play` _sound _start_time)))
        (set `self.Is Fading Out` false))
      (else
        (goto _label)))))

(fn `Stop Audio`
  (if (`self.Enabled`)
    (`AudioComponent.StopDelayed` (`self.Sound`) (`self.Stop Delay Time`))))

(fn `UserConstructionScript`)
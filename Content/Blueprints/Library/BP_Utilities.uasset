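; Blueprint function library of shared lookup helpers for Paper Golf.
; Getters cast the game state and the local player, controller and player state to their Paper Golf types.
; A debug-draw check builds on the controller getter, querying the controller's setting only in non-shipping builds when that controller is valid.
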(fn `Get Paper Golf Game State`
  (returns (`Golf Game State` :type "PaperGolfGameStateBase Object Reference"))
  (bind _aspaper_golf_game_state_base (cast `PaperGolfGameStateBase` (`GameplayStatics.GetGameState` null)))
  (return _aspaper_golf_game_state_base))

(fn `Get Paper Golf Pawn`
  (returns (`Paper Golf Pawn` :type "PaperGolfPawn Object Reference"))
  (bind _aspaper_golf_pawn (cast `PaperGolfPawn` (`PaperGolfGameUtilities.GetLocalPlayer` null)))
  (return _aspaper_golf_pawn))

(fn `Get Paper Golf Player Controller`
  (returns (`Golf Player Controller` :type "/Game/Blueprints/Player/BP_PaperGolfPlayerController Object Reference"))
  (bind _asbp_paper_golf_player_controller (cast `/Game/Blueprints/Player/BP_PaperGolfPlayerController` (`PaperGolfGameUtilities.GetLocalPlayerController` null)))
  (return _asbp_paper_golf_player_controller))

(fn `Get Paper Golf Player State`
  (returns (`Golf Player State` :type "GolfPlayerState Object Reference"))
  (bind _asgolf_player_state (cast `GolfPlayerState` (`PaperGolfGameUtilities.GetLocalPlayerState` null)))
  (return _asgolf_player_state))

(fn `Is Debug Draw Enabled`
  (returns (`Debug Draw Enabled` :type Boolean))
  (bind _golf_player_controller (`self.Get Paper Golf Player Controller` null))
  (if (`BuildUtilities.IsNotShipping`)
    (`/Engine/EditorBlueprintResources/StandardMacros.IsValid` _golf_player_controller
      (:`Is Valid`
        (return (`/Game/Blueprints/Player/BP_PaperGolfPlayerController.Is Debug Draw Enabled` _golf_player_controller))))))